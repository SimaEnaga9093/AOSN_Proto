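; BP_GameModeBattle is a battle game mode that builds a tile grid and places a unit on it at BeginPlay.
; InitBattle fills MapData with zeros and spawns a BP_TileBase per cell, labeling each with its grid coordinates.
; InitUnit converts grid coordinates to world space via TileLength and spawns a raised BP_UnitBase, called once for a non-ally.
; The IsAlly input is currently unused.
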(event EventBeginPlay
  (|CallParentFunction)
  (CallFunction|InitBattle)
  (CallFunction|InitUnit false 5 8))

(fn ConstructionScript)

(fn InitBattle
  (Variables|Default|SetMapData (Utilities|Array|MakeArray))
  (for _index (range 0 (- (LocalVariables|GetMapWidth) 1))
    (for _index_2 (range 0 (- (LocalVariables|GetMapHeight) 1))
      (Utilities|Array|Add (Variables|Default|GetMapData) 0)
      (bind _returnvalue (Game|SpawnActorfromClass "/Game/Battle/Blueprint/BP_TileBase.BP_TileBase_C" (Math|Transform|MakeTransform (Math|Vector|MakeVector (* _index (Variables|Default|GetTileLength)) (* _index_2 (Variables|Default|GetTileLength)) 0.0)) "AlwaysSpawn" "MultiplyWithRoot" 0 0))
      (Rendering|Components|TextRender|SetText (Variables|/Game/Battle/Blueprint/BP_TileBase.BP_TileBase_C|GetTextPos _returnvalue) (Utilities|Text|FormatText "({X},{Y})" _index _index_2)))))

(fn InitUnit
  (params (IsAlly :type Boolean) (StartX :type Integer) (StartY :type Integer))
  (Game|SpawnActorfromClass "/Game/Battle/Blueprint/BP_UnitBase.BP_UnitBase_C" (Math|Transform|MakeTransform (Math|Vector|MakeVector (* StartX (Variables|Default|GetTileLength)) (* StartY (Variables|Default|GetTileLength)) 2e+01)) "AlwaysSpawn" "MultiplyWithRoot" 0 0))