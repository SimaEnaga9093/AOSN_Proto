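; Base Blueprint for grid battle units that span a set of tile positions and move toward their own spawned flag actor.
; On BeginPlay it centers the skeletal mesh on the tile bounds using the game mode's tile length, then spawns the flag with matching offset and positions.
; UpdateLocationToFlag steps the unit toward the flag by MoveSpeed per call, smoothing mesh rotation and setting IsMove.
; Tick only calls its parent.
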(event EventBeginPlay
  (|CallParentFunction)
  (CallFunction|UpdateMeshtoCenter)
  (bind _returnvalue (Game|SpawnActorfromClass "/Game/Battle/Blueprint/Unit/BP_UnitBase_Flag.BP_UnitBase_Flag_C" (Transformation|GetActorTransform) "AlwaysSpawn" "MultiplyWithRoot" self 0))
  (bind _output_get (Variables|Default|SetFlag _returnvalue))
  (Transformation|AddRelativeLocation (Variables|/Game/Battle/Blueprint/Unit/BP_UnitBase_Flag.BP_UnitBase_Flag_C|GetCylinder _output_get) (Variables|Default|GetCenterRelativeLocation) false true)
  (Variables|/Game/Battle/Blueprint/Unit/BP_UnitBase_Flag.BP_UnitBase_Flag_C|SetPosInfos _output_get (Variables|Default|GetPosInfos)))

(event EventTick
  (params (DeltaSeconds :type Float%20%28single-precision%29))
  (|CallParentFunction DeltaSeconds))

(fn ConstructionScript)

(fn UpdateMeshtoCenter
  (for _array_element (Variables|Default|GetPosInfos)
    (Utilities|FlowControl|Sequence
      (:then_0
        (if (> (LocalVariables|GetMinX) (.x _array_element))
          (LocalVariables|SetMinX (.x _array_element))
          (elif (< (LocalVariables|GetMaxX) (.x _array_element))
            (LocalVariables|SetMaxX (.x _array_element)))))
      (:then_1
        (if (> (LocalVariables|GetMinY) (.y _array_element))
          (LocalVariables|SetMinY (.y _array_element))
          (elif (< (LocalVariables|GetMaxY) (.y _array_element))
            (LocalVariables|SetMaxY (.y _array_element)))))))
  (bind _asbp_game_mode_battle (Utilities|Casting|CastToBP_GameModeBattle (Game|GetGameMode)))
  (bind _output_get (Variables|Default|SetCenterRelativeLocation (* (Variables|/Game/Battle/Blueprint/Base/BP_GameModeBattle.BP_GameModeBattle_C|GetTileLength _asbp_game_mode_battle) (Math|Vector|MakeVector (|((({23423EA3-4A59-63D8-5261-3D8E53DE1BF9}-{3AF03A64-4BF5-E740-F095-2CB909C386D9})/2)+{3AF03A64-4BF5-E740-F095-2CB909C386D9})) (|((({2F1D7A8E-4B17-5B2B-792E-548F7637E5ED}-{2B11B8CB-41A1-19FC-B72C-3EBF725A4FAA})/2)+{2B11B8CB-41A1-19FC-B72C-3EBF725A4FAA})) 0.0))))
  (Transformation|SetRelativeLocation (Variables|Default|GetSkeletalMesh) _output_get false true))

(fn UpdateLocationtoFlag
  (bind _returnvalue (Transformation|GetActorLocation))
  (bind _flag (Variables|Default|GetFlag))
  (bind _skeletalmesh (Variables|Default|GetSkeletalMesh))
  (bind _returnvalue_2 (Transformation|GetActorLocation _flag))
  (bind _returnvalue_3 (Math|Rotator|FindLookatRotation _returnvalue _returnvalue_2))
  (if (> (Math|Vector|Distance(Vector) (Transformation|GetActorLocation) (Transformation|GetActorLocation (Variables|Default|GetFlag))) (Utilities|Struct|BreakS_UnitStat (Variables|Default|GetUnitStat)))
    (Transformation|SetActorLocation (+ _returnvalue (* (Math|Vector|GetForwardVector _returnvalue_3) (Utilities|Struct|BreakS_UnitStat (Variables|Default|GetUnitStat)))) true false)
    (Transformation|SetRelativeRotation _skeletalmesh (Math|Rotator|Lerp(Rotator) (Transformation|GetWorldRotation _skeletalmesh) (Math|Rotator|CombineRotators _returnvalue_3 "0.000000,-90.000000,0.000000") 0.5) false false)
    (Variables|Default|SetIsMove true)
    (else
      (Variables|Default|SetIsMove false))))