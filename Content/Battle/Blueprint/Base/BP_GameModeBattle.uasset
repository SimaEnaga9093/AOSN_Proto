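; Battle game mode that builds a grid map of tiles on BeginPlay, spawns four test allied units and moves the player pawn.
; InitBattle fills MapData per cell and spawns labeled tiles, while InitUnit places units with stats and a flag position.
; Helpers convert between grid and world coordinates, find allies by multi-cell footprint at unit or flag position, and move flags only onto cells valued zero in MapData.
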(event EventTick
  (params (DeltaSeconds :type Float%20%28single-precision%29))
  (|CallParentFunction DeltaSeconds))

(event EventBeginPlay
  (|CallParentFunction)
  (CallFunction|InitBattle)
  (CallFunction|InitUnit true "(X=5.000000,Y=8.000000)" (Utilities|Struct|MakeS_UnitStat 1e+02 1e+02 1e+02 1.0 1.0 1.0 1e+01 0.0 0.0 1e+01 5.0 5.0 5.0 1.0))
  (CallFunction|InitUnit true "(X=8.000000,Y=5.000000)" (Utilities|Struct|MakeS_UnitStat 1e+02 1e+02 1e+02 1.0 1.0 1.0 1e+01 0.0 0.0 1e+01 5.0 5.0 5.0 1.0))
  (CallFunction|InitUnit true "(X=5.000000,Y=5.000000)" (Utilities|Struct|MakeS_UnitStat 1e+02 1e+02 1e+02 1.0 1.0 1.0 1e+01 0.0 0.0 1e+01 5.0 5.0 5.0 1.0))
  (CallFunction|InitUnit true "(X=8.000000,Y=8.000000)" (Utilities|Struct|MakeS_UnitStat 1e+02 1e+02 1e+02 1.0 1.0 1.0 1e+01 0.0 0.0 1e+01 5.0 5.0 5.0 1.0))
  (Transformation|SetActorLocation (Game|Player|GetPlayerPawn 0) (Math|Vector|MakeVector (|(({FE2D7FE4-4075-84DA-1278-78B19045E777}*{6CDCFCF5-484A-E06C-AD6C-F28DBDE2FA51})/2)) (|(({D914D670-4484-A9DF-114F-09AA3805B1D4}*{6CDCFCF5-484A-E06C-AD6C-F28DBDE2FA51})/2)) 0.0) false false))

(fn ConstructionScript)

(fn InitBattle
  (Variables|Default|SetMapData (Utilities|Map|MakeMap))
  (for _index (range 0 (- (Variables|Default|GetMapWidth) 1))
    (for _index_2 (range 0 (- (Variables|Default|GetMapHeight) 1))
      (Utilities|Map|Add (Variables|Default|GetMapData) (Math|Vector2D|MakeVector2D (Math|Conversions|ToFloat(Integer) _index) (Math|Conversions|ToFloat(Integer) _index_2)) 0)
      (bind _returnvalue (Game|SpawnActorfromClass "/Game/Battle/Blueprint/BP_TileBase.BP_TileBase_C" (Math|Transform|MakeTransform (Math|Vector|MakeVector (* _index (Variables|Default|GetTileLength)) (* _index_2 (Variables|Default|GetTileLength)) 0.0)) "AlwaysSpawn" "MultiplyWithRoot" 0 0))
      (Variables|/Game/Battle/Blueprint/BP_TileBase.BP_TileBase_C|SetPos _returnvalue (Math|Vector2D|MakeVector2D (Math|Conversions|ToFloat(Integer) _index) (Math|Conversions|ToFloat(Integer) _index_2)))
      (Rendering|Components|TextRender|SetText (Variables|/Game/Battle/Blueprint/BP_TileBase.BP_TileBase_C|GetTextPos _returnvalue) (Utilities|Text|FormatText "({X},{Y})" _index _index_2)))))

(fn InitUnit
  (params (IsAlly :type Boolean) (StartPos :type Vector%202D%20Structure) (UnitStat :type S%20Unit%20Stat%20Structure))
  (bind _outvec (CallFunction|PostoWorld StartPos))
  (bind _returnvalue (Game|SpawnActorfromClass "/Game/Battle/Blueprint/Unit/BP_UnitBase.BP_UnitBase_C" (Math|Transform|MakeTransform (+ _outvec "0.000000,0.000000,20.000000") "0, 0, 0" "1.000000,1.000000,1.000000") "AlwaysSpawn" "MultiplyWithRoot" 0 0))
  (Utilities|Array|Add (Variables|Default|GetAllyUnits) _returnvalue)
  (Variables|/Game/Battle/Blueprint/Unit/BP_UnitBase.BP_UnitBase_C|SetCurrentCenterPos _returnvalue StartPos)
  (Variables|/Game/Battle/Blueprint/Unit/BP_UnitBase_Flag.BP_UnitBase_Flag_C|SetCurrentPos (Variables|/Game/Battle/Blueprint/Unit/BP_UnitBase.BP_UnitBase_C|GetFlag _returnvalue) StartPos)
  (Variables|/Game/Battle/Blueprint/Unit/BP_UnitBase.BP_UnitBase_C|SetUnitStat _returnvalue UnitStat))

(fn GetAllyUnitonPos
  (params (TargetPos :type Vector%202D%20Structure) (UseFlagPos :type Boolean))
  (bind _array_element (Utilities|Array|ForEachLoopwithBreak (Variables|Default|GetAllyUnits))
    (:LoopBody
      (Utilities|FlowControl|Sequence
        (:then_0
          (if UseFlagPos
            (LocalVariables|SetTargetPos2D (Variables|/Game/Battle/Blueprint/Unit/BP_UnitBase_Flag.BP_UnitBase_Flag_C|GetCurrentPos (Variables|/Game/Battle/Blueprint/Unit/BP_UnitBase.BP_UnitBase_C|GetFlag _array_element)))
            (else
              (LocalVariables|SetTargetPos2D (Variables|/Game/Battle/Blueprint/Unit/BP_UnitBase.BP_UnitBase_C|GetCurrentCenterPos _array_element)))))
        (:then_1
          (bind _array_element_2 (Utilities|Array|ForEachLoopwithBreak (Variables|/Game/Battle/Blueprint/Unit/BP_UnitBase.BP_UnitBase_C|GetPosInfos _array_element))
            (:LoopBody
              (if (Utilities|Operators|EqualEqual TargetPos (+ _array_element_2 (LocalVariables|GetTargetPos2D)) 0.0)
                (return true _array_element)))))))
    (:Completed
      (return false 0))))

(fn PostoWorld
  (params (InPos :type Vector%202D%20Structure))
  (return (Math|Vector|MakeVector (* (.x InPos) (Variables|Default|GetTileLength)) (* (.y InPos) (Variables|Default|GetTileLength)) 0.0)))

(fn WorldtoPos
  (params (InVec :type Vector))
  (return (Math|Vector2D|MakeVector2D (Math|Conversions|ToFloat(Integer) (/ (.x InVec) (Variables|Default|GetTileLength))) (Math|Conversions|ToFloat(Integer) (/ (.y InVec) (Variables|Default|GetTileLength))))))

(fn MoveFlagtoPos
  (params (TargetFlag :type BP%20Unit%20Base%20Flag%20Object%20Reference) (TargetPos :type Vector%202D%20Structure))
  (bind _array_element (Utilities|Array|ForEachLoopwithBreak (Variables|/Game/Battle/Blueprint/Unit/BP_UnitBase_Flag.BP_UnitBase_Flag_C|GetPosInfos TargetFlag))
    (:LoopBody
      (if (!= (.Value (Utilities|Map|Find (Variables|Default|GetMapData) (+ _array_element TargetPos))) 0)
        (return false)))
    (:Completed
      (Variables|/Game/Battle/Blueprint/Unit/BP_UnitBase_Flag.BP_UnitBase_Flag_C|SetCurrentPos TargetFlag TargetPos)
      (return true))))