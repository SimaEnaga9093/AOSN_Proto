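; Battle player controller that lets the player click and drag an allied unit's flag across the tile grid.
; Left press traces under the cursor for a tile and grabs the ally whose flag position matches it; release clears the selection.
; While held, Tick re-traces and moves the flag to the hovered tile's world position, skipping the start tile and tiles held by other allies.
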(event EventBeginPlay
  (|CallParentFunction))

(event EventTick
  (params (DeltaSeconds :type Float%20%28single-precision%29))
  (|CallParentFunction DeltaSeconds)
  (if (Math|Boolean|ANDBoolean (Variables|Default|GetbIsClicked) (Utilities|IsValid (Variables|Default|GetClickedUnitBase)) (Utilities|Enum|Equal(Enum) (Variables|Default|GetCurrentInputMode) "NewEnumerator1"))
    (bind _outhits (CallFunction|TraceMousePosition "TraceTypeQuery3"))
    (bind _array_element (Utilities|Array|ForEachLoopwithBreak _outhits :!label _label)
      (:LoopBody
        (bind _asbp_tile_base (Utilities|Casting|CastToBP_TileBase (.HitActor (Collision|BreakHitResult _array_element))))
        (if (Utilities|Operators|NotEqual(!=) (Variables|/Game/Battle/Blueprint/BP_TileBase.BP_TileBase_C|GetPos _asbp_tile_base) (Variables|Default|GetClickedStartPos) 0.0)
          (bind _gamemodebattle (CallFunction|GetGameModeBattle self))
          (bind (_isin _outunitbase) (Default|GetAllyUnitonPos _gamemodebattle (Variables|/Game/Battle/Blueprint/BP_TileBase.BP_TileBase_C|GetPos _asbp_tile_base) true))
          (if _isin
            (if (== _outunitbase (Variables|Default|GetClickedUnitBase))
              _
              (else
                (goto _label Break))))
          (bind _outvec (Default|PostoWorld _gamemodebattle (Variables|/Game/Battle/Blueprint/BP_TileBase.BP_TileBase_C|GetPos _asbp_tile_base)))
          (Default|UpdateClickLocation (Variables|/Game/Battle/Blueprint/Unit/BP_UnitBase.BP_UnitBase_C|GetFlag (Variables|Default|GetClickedUnitBase)) _outvec)
          (goto _label Break))))))

(event Input|MouseEvents|LeftMouseButton
  (params (Key :type Key%20Structure :default "None"))
  (:Pressed
    (Variables|Default|SetbIsClicked true)
    (bind _outhits (CallFunction|TraceMousePosition "TraceTypeQuery3"))
    (bind _array_element (Utilities|Array|ForEachLoopwithBreak _outhits)
      (:LoopBody
        (bind _asbp_tile_base (Utilities|Casting|CastToBP_TileBase (.HitActor (Collision|BreakHitResult _array_element))))
        (bind _gamemodebattle (CallFunction|GetGameModeBattle self))
        (bind (_isin _outunitbase) (Default|GetAllyUnitonPos _gamemodebattle (Variables|/Game/Battle/Blueprint/BP_TileBase.BP_TileBase_C|GetPos _asbp_tile_base) true))
        (if _isin
          (Variables|Default|SetCurrentInputMode "NewEnumerator1")
          (Variables|Default|SetClickedUnitBase _outunitbase)
          (Variables|Default|SetClickedStartPos (Variables|/Game/Battle/Blueprint/BP_TileBase.BP_TileBase_C|GetPos _asbp_tile_base))))))
  (:Released
    (Variables|Default|SetbIsClicked false)
    (Variables|Default|SetCurrentInputMode "NewEnumerator0")
    (Variables|Default|SetClickedUnitBase 0)
    (Variables|Default|SetClickedStartPos "")))

(fn ConstructionScript)

(fn TraceMousePosition
  (params (TraceChannel :type ETraceTypeQuery%20Enum :default "TraceTypeQuery3"))
  (bind _returnvalue (Game|GetPlayerController 0))
  (bind (_worldlocation _worlddirection) (Game|Player|ConvertMouseLocationToWorldSpace _returnvalue))
  (bind _outhits (Collision|MultiLineTraceByChannel _worldlocation (+ _worldlocation (* _worlddirection 1e+04)) TraceChannel false 0 "None"))
  (return _outhits))